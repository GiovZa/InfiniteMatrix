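; BP_HealthPack is a short-lived health pickup that destroys itself five seconds after BeginPlay.
; When BP_Player overlaps its Collide component, it adds a fixed amount to PlayerHealth, capped at full, then destroys itself and plays a munch sound.
; The construction script creates a dynamic instance of MI_HealthPack and sets a red vector parameter, but does not assign it to a component.
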(event `self.ReceiveBeginPlay`
  (`KismetSystemLibrary.Delay` 5.0)
  (`self.K2_DestroyActor`))

(event `self.Collide.OnComponentBeginOverlap`
  (params (OverlappedComponent :type "PrimitiveComponent Object Reference") (OtherActor :type "Actor Object Reference") (OtherComp :type "PrimitiveComponent Object Reference") (OtherBodyIndex :type Integer) (bFromSweep :type Boolean) (SweepResult :type "HitResult Structure (by ref)"))
  (bind _returnvalue_location (`KismetMathLibrary.BreakTransform` (`self.GetTransform`)))
  (bind _asbp_player (cast `/Game/InfiniteMatrix/Blueprints/BP_Player` OtherActor))
  (set `/Game/InfiniteMatrix/Blueprints/BP_Player.PlayerHealth` (`KismetMathLibrary.FMin` (+ (`/Game/InfiniteMatrix/Blueprints/BP_Player.PlayerHealth` _asbp_player) 0.2) 1.0) _asbp_player)
  (`self.K2_DestroyActor`)
  (`GameplayStatics.PlaySoundAtLocation` "/Game/InfiniteMatrix/Sounds/S_Munch.S_Munch" _returnvalue_location (struct) 1.0 1.0 0.0 null null null null))

(fn `UserConstructionScript`
  (locals (NewLocalVar :type Name :default "None"))
  (bind _returnvalue (`KismetMaterialLibrary.CreateDynamicMaterialInstance` "/Game/InfiniteMatrix/Materials/MI_HealthPack.MI_HealthPack"))
  (`MaterialInstanceDynamic.SetVectorParameterValue` _returnvalue (`local.NewLocalVar`) (make `LinearColor` 1.0)))
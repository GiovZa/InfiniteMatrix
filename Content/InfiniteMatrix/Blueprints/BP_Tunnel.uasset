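; BP_Tunnel is a tunnel segment with a rotating wall obstacle, used in an endlessly spawned tunnel course.
; Its wall rolls at a randomized speed and direction, and RandomizeWall can pick a hole mesh and starting roll.
; Crossing the trigger spawns another tunnel, destroys this one and adds score.
; Hitting the wall disables its collision, cuts score and player health toward death, while overlapping actors are destroyed with a bullet-hit sound.
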(event `self.ReceiveBeginPlay`
  (set `self.RotateSpeed` (* (`self.RotateSpeed`) (`KismetArrayLibrary.Array_Random` (`|MakeArray` (`KismetMathLibrary.RandomFloatInRange` -2.0 -1.0) (`KismetMathLibrary.RandomFloatInRange` 1.0 2.0))))))

(event `self.ReceiveTick`
  (params (DeltaSeconds :type "Float (single-precision)"))
  (`SceneComponent.K2_AddLocalRotation` (`self.WallMesh`) (`KismetMathLibrary.MakeRotator` (* DeltaSeconds (`self.RotateSpeed`))) false false))

(event `self.TriggerZone.OnComponentBeginOverlap`
  (params (OverlappedComponent :type "PrimitiveComponent Object Reference") (OtherActor :type "Actor Object Reference") (OtherComp :type "PrimitiveComponent Object Reference") (OtherBodyIndex :type Integer) (bFromSweep :type Boolean) (SweepResult :type "HitResult Structure (by ref)"))
  (cast `/Game/InfiniteMatrix/Blueprints/BP_Player` OtherActor)
  (`/Game/InfiniteMatrix/Blueprints/BP_TunnelSpawner.SpawnTunnelAtSpawnPoint` (`self.TunnelSpawner`))
  (`self.K2_DestroyActor`)
  (bind _foundwidgets (`WidgetBlueprintLibrary.GetAllWidgetsOfClass` "/Game/InfiniteMatrix/UI/WBP_Score.WBP_Score_C" false))
  (for _array_element _foundwidgets
    (set `/Game/InfiniteMatrix/UI/WBP_Score.Score` (+ (`/Game/InfiniteMatrix/UI/WBP_Score.Score` _array_element) 5.0) _array_element)))

(event `self.WallMesh.OnComponentHit`
  (params (HitComponent :type "PrimitiveComponent Object Reference") (OtherActor :type "Actor Object Reference") (OtherComp :type "PrimitiveComponent Object Reference") (NormalImpulse :type "Vector Structure") (Hit :type "HitResult Structure (by ref)"))
  (bind _asbp_player (cast `/Game/InfiniteMatrix/Blueprints/BP_Player` OtherActor))
  (`PrimitiveComponent.SetCollisionEnabled` HitComponent "NoCollision")
  (bind _output_get (set `/Game/InfiniteMatrix/Blueprints/BP_Player.PlayerHealth` (- (`/Game/InfiniteMatrix/Blueprints/BP_Player.PlayerHealth` _asbp_player) 0.34) _asbp_player))
  (bind _foundwidgets (`WidgetBlueprintLibrary.GetAllWidgetsOfClass` "/Game/InfiniteMatrix/UI/WBP_Score.WBP_Score_C"))
  (for _array_element _foundwidgets
    (set `/Game/InfiniteMatrix/UI/WBP_Score.Score` (- (`/Game/InfiniteMatrix/UI/WBP_Score.Score` _array_element) 5.0) _array_element)
    (if (<= _output_get 0.01)
      (set `/Game/InfiniteMatrix/Blueprints/BP_Player.IsDead` true _asbp_player)
      (`/Game/InfiniteMatrix/Blueprints/BP_Player.DisplayRestart` _asbp_player))))

(event `self.WallMesh.OnComponentBeginOverlap`
  (params (OverlappedComponent :type "PrimitiveComponent Object Reference") (OtherActor :type "Actor Object Reference") (OtherComp :type "PrimitiveComponent Object Reference") (OtherBodyIndex :type Integer) (bFromSweep :type Boolean) (SweepResult :type "HitResult Structure (by ref)"))
  (`self.K2_DestroyActor` OtherActor)
  (`GameplayStatics.PlaySoundAtLocation` "/Game/InfiniteMatrix/Sounds/S_Bullet_Hit.S_Bullet_Hit" (`SceneComponent.K2_GetComponentLocation` (`self.WallMesh`)) (struct) 1.0 1.0 0.0 null null null null))

(fn `RandomizeWall`
  (`StaticMeshComponent.SetStaticMesh` (`self.WallMesh`) (select `int` (`KismetMathLibrary.RandomIntegerInRange` 0 3) :`0` "/Game/InfiniteMatrix/Meshes/SM_Hole_01.SM_Hole_01" :`1` "/Game/InfiniteMatrix/Meshes/SM_Hole_02.SM_Hole_02" :`2` "/Game/InfiniteMatrix/Meshes/SM_Hole_02.SM_Hole_02" :`3` "/Game/InfiniteMatrix/Meshes/SM_Hole_04.SM_Hole_04" :!type "StaticMesh Object Reference"))
  (`SceneComponent.K2_AddLocalRotation` (`self.WallMesh`) (`KismetMathLibrary.MakeRotator` (`KismetMathLibrary.RandomFloatInRange` 0.0 360.0)) false false))

(fn `UserConstructionScript`)
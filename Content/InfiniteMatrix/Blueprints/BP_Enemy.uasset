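; BP_Enemy is a short-lived enemy actor that destroys itself five seconds after spawning.
; Overlap with BP_Projectile plays a hit sound, destroys the enemy and adds points directly to every top-level WBP_Score widget.
; A Collision_Spike hit on BP_Player reduces health, clamped at zero, plays a hurt sound, destroys the enemy and calls DisplayRestart when health runs out.
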(event `self.ReceiveBeginPlay`
  (`KismetSystemLibrary.Delay` 5.0)
  (`self.K2_DestroyActor`))

(event `self.ReceiveActorBeginOverlap`
  (params (OtherActor :type "Actor Object Reference"))
  (bind _returnvalue_location (`KismetMathLibrary.BreakTransform` (`self.GetTransform`)))
  (cast `/Game/InfiniteMatrix/Blueprints/BP_Projectile` OtherActor)
  (`GameplayStatics.PlaySoundAtLocation` "/Game/InfiniteMatrix/Sounds/S_Bullet_Hit.S_Bullet_Hit" _returnvalue_location (struct) 1.0 1.0 0.0 null null null null)
  (`self.K2_DestroyActor`)
  (bind _foundwidgets (`WidgetBlueprintLibrary.GetAllWidgetsOfClass` "/Game/InfiniteMatrix/UI/WBP_Score.WBP_Score_C"))
  (for _array_element _foundwidgets
    (set `/Game/InfiniteMatrix/UI/WBP_Score.Score` (+ (`/Game/InfiniteMatrix/UI/WBP_Score.Score` _array_element) 5.0) _array_element)))

(event `self.Collision_Spike.OnComponentHit`
  (params (HitComponent :type "PrimitiveComponent Object Reference") (OtherActor :type "Actor Object Reference") (OtherComp :type "PrimitiveComponent Object Reference") (NormalImpulse :type "Vector Structure") (Hit :type "HitResult Structure (by ref)"))
  (bind _returnvalue_location (`KismetMathLibrary.BreakTransform` (`self.GetTransform`)))
  (bind _asbp_player (cast `/Game/InfiniteMatrix/Blueprints/BP_Player` OtherActor))
  (bind _playerhealth (`/Game/InfiniteMatrix/Blueprints/BP_Player.PlayerHealth` _asbp_player))
  (set `/Game/InfiniteMatrix/Blueprints/BP_Player.PlayerHealth` (`KismetMathLibrary.FMax` (- _playerhealth 0.25)) _asbp_player)
  (`GameplayStatics.PlaySoundAtLocation` "/Game/InfiniteMatrix/Sounds/S_Player_Hit.S_Player_Hit" _returnvalue_location (struct) 1.0 1.0 0.0 null null null null)
  (`self.K2_DestroyActor`)
  (if (<= _playerhealth 0.0)
    (`/Game/InfiniteMatrix/Blueprints/BP_Player.DisplayRestart` _asbp_player)))

(fn `UserConstructionScript`)